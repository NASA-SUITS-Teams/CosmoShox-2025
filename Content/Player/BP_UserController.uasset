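; Player controller that shows the HUD root layout, monitors EV telemetry and handles mouse-wheel map zoom and Escape to quit.
; BeginPlay seeds telemetry from DT_Telemetry2025 and, inside that row loop, starts an ObjectDeliverer TCP client that prints received strings.
; CheckTelemetry polls Connection's JSON every two seconds, comparing values against each row's limits.
; New out-of-range values create warning messages and push the warning screen, with ShownWarning suppressing repeats until nominal.
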(event `Connected Event`
  (params (ClientSocket :type "ObjectDelivererProtocol Object Reference"))
  (`KismetSystemLibrary.PrintString` "Connected!"))

(event `Disconnected Event`
  (params (ClientSocket :type "ObjectDelivererProtocol Object Reference"))
  (`KismetSystemLibrary.PrintString` "Disconnected!"))

(event `self.ReceiveBeginPlay`
  (bind _connection (`self.Connection`))
  ; Create the Root Layout and show it to screen
  (bind _returnvalue (`|CreateWidget` "/Game/UI/WBP_RootLayout.WBP_RootLayout_C" self))
  (bind _output_get (set `self.Root Layout` _returnvalue))
  (`UserWidget.AddToViewport` _output_get 0)
  (`/Game/UI/WBP_RootLayout.PushWidgetToLayerStack` (`self.Root Layout`) (struct :`TagName` "UI.Layer.Menu") (`self.HUD Layout Class`))
  (`WidgetBlueprintLibrary.SetInputMode_GameAndUIEx` self null)
  ; Initialize The array of data for each point of telemetry.
  (bind _outrownames (`DataTableFunctionLibrary.GetDataTableRowNames` "/Game/Player/Data/DT_Telemetry2025.DT_Telemetry2025"))
  (for (_array_element _array_index) _outrownames
    (bind _returnvalue_2 (`|GetDataTableRow` "/Game/Player/Data/DT_Telemetry2025.DT_Telemetry2025" _array_element)
      (:`then`
        (`KismetArrayLibrary.Array_Set` (`self.FTelemetry Data`) _array_index (make `/Game/Player/Data/FTelemetryData` (break `/Game/Player/Data/FTelemetryData` _returnvalue_2) (`.VarName_12_6EFAEC1249BC4487FA7D6CB2912D0B2D` (break `/Game/Player/Data/FTelemetryData` _returnvalue_2)) (`.Value_7_1C4A3E064C87644618BD699E1D85A286` (break `/Game/Player/Data/FTelemetryData` _returnvalue_2)) (`.Minimum_9_51847DF84CBE4681A7B6C2B64405C49A` (break `/Game/Player/Data/FTelemetryData` _returnvalue_2)) (`.Maximum_11_C0653E58444A9EB6FE7C6A95938BB0D2` (break `/Game/Player/Data/FTelemetryData` _returnvalue_2)) (`.Units_19_6F8C2E2845B0107184B24E8952736842` (break `/Game/Player/Data/FTelemetryData` _returnvalue_2)) (`.Warning_21_4B708D78436292F8CE8EE6823ECD9DA2` (break `/Game/Player/Data/FTelemetryData` _returnvalue_2)) (`.ShownWarning_23_879702BA4D657414B35F0C8514E71E51` (break `/Game/Player/Data/FTelemetryData` _returnvalue_2)) (`.ShortenedNames_26_885F838C4306A0CA160422B90A963794` (break `/Game/Player/Data/FTelemetryData` _returnvalue_2))) true)
        (`|ExecutionSequence`
          (:`then_0`
            (bind _output_get_2 (set `self.Deliverer` (`ObjectDelivererManager.CreateObjectDelivererManager` true)))
            (add `ObjectDelivererManager.Connected` _output_get_2 (delegate `Connected Event`))
            (add `ObjectDelivererManager.Disconnected` _output_get_2 (delegate `Disconnected Event`)))
          (:`then_1`
            (bind _output_get_3 (set `self.DeliveryBox` (`DeliveryBoxFactory.CreateUtf8StringDeliveryBox`)))
            (add `Utf8StringDeliveryBox.Received` _output_get_3 (delegate `Received Event 1`)))
          (:`then_2`
            (`ObjectDelivererManager.Start` (`self.Deliverer`) (`ProtocolFactory.CreateProtocolTcpIpClient` (`/Game/TSS/TSS_Connection.url` _connection) (`KismetStringLibrary.Conv_StringToInt` (`/Game/TSS/TSS_Connection.port` _connection)) true true) (`PacketRuleFactory.CreatePacketRuleSizeBody` 4) (`self.DeliveryBox`)))))))
  (`self.Check Telemetry`))

(event `Received Event 1`
  (params (ReceivedString :type String) (FromObject :type "ObjectDelivererProtocol Object Reference"))
  (`KismetSystemLibrary.PrintString` ReceivedString))

(event `Get Lidar`
  (`Utf8StringDeliveryBox.Send` (`self.DeliveryBox`) "165"))

(event `Check Telemetry`
  (bind _connection (`self.Connection`))
  (`|ExecutionSequence`
    (:`then_0`
      (bind _uia_updated (`/Game/TSS/TSS_Connection.IsTELEMETRYUpdated` _connection))
      (if _uia_updated
        (`KismetSystemLibrary.PrintString` "Checking Telemetry")
        ; Get the Current Telemetry
        (bind _uia_json_string (`/Game/TSS/TSS_Connection.GetTELEMETRYJsonString` _connection))
        (bind _jsonobject (`EasyJsonAsyncLoadFromString.AsyncLoadFromString` _uia_json_string)
          (:`Successed`
            (set `self.TELEMETRY Json Object` _jsonobject)
            ; For each row in the data table, update the row with current telemetry data
            (bind _outrownames (`DataTableFunctionLibrary.GetDataTableRowNames` "/Game/Player/Data/DT_Telemetry2025.DT_Telemetry2025"))
            (for (_array_element _array_index) _outrownames
              (bind _returnvalue (`|GetDataTableRow` "/Game/Player/Data/DT_Telemetry2025.DT_Telemetry2025" _array_element)
                (:`then`
                  (bind (_evname _varname _value _minimum _maximum _units _warning _shownwarning _shortenednames _humanreadablenames) (break `/Game/Player/Data/FTelemetryData` _returnvalue))
                  (bind _returnvalue_2 (`EasyJsonObject.ReadFloat` (`self.TELEMETRY Json Object`) (`KismetStringLibrary.Concat_StrStr` "telemetry" "." _evname "." _varname) 98.0))
                  (bind _returnvalue_3 (or (< _returnvalue_2 _minimum) (> _returnvalue_2 _maximum)))
                  (if _returnvalue_3
                    (bind (_output_evname _output_varname _output_value _output_minimum _output_maximum _output_units _output_warning _output_shownwarning) (break `/Game/Player/Data/FTelemetryData` (`|GetArrayItem` (`self.FTelemetry Data`) _array_index)))
                    (if (not _output_shownwarning)
                      (set `self.bShowWarningScreen` true)
                      (set `self.bAddWarningMessage` true))
                    (bind (_output_evname_2 _output_varname_2 _output_value_2 _output_minimum_2 _output_maximum_2 _output_units_2 _output_warning_2 _output_shownwarning_2 _output_shortenednames) (break `/Game/Player/Data/FTelemetryData` (`|GetArrayItem` (`self.FTelemetry Data`) _array_index)))
                    (`KismetArrayLibrary.Array_Set` (`self.FTelemetry Data`) _array_index (make `/Game/Player/Data/FTelemetryData` _output_evname_2 _output_varname_2 _returnvalue_2 _output_minimum_2 _output_maximum_2 _output_units_2 _returnvalue_3 true _output_shortenednames _humanreadablenames) true)
                    (if (`self.bAddWarningMessage`)
                      (set `self.bAddWarningMessage` false)
                      ; Lastly, Create a warning message to add the warning screen using the data from this telemetry...
                      (bind _returnvalue_4 (`|CreateWidget` "/Game/UI/Foundation/Widgets/WBP_WarningMessage.WBP_WarningMessage_C"))
                      (`TextBlock.SetText` (`/Game/UI/Foundation/Widgets/WBP_WarningMessage.Message` _returnvalue_4) (`|GenericToText` (`KismetStringLibrary.Concat_StrStr` _humanreadablenames " outside nominal ranges!")))
                      (`KismetArrayLibrary.Array_Set` (`self.Warning Message`) _array_index _returnvalue_4 true))
                    (else
                      ; If there is no warning, just set the value and close the loop for this array member.
                      (`KismetArrayLibrary.Array_Set` (`self.FTelemetry Data`) _array_index (make `/Game/Player/Data/FTelemetryData` _evname _varname _returnvalue_2 _minimum _maximum _units _returnvalue_3 false _shortenednames _humanreadablenames) true))))))
            ; Once the For Each Loop is complete, if there is a warning, push the warning widget to the stack. If there is no warning continue on
            (if (`self.bShowWarningScreen`)
              (set `self.bShowWarningScreen` false)
              (`KismetSystemLibrary.PrintString` "I SHOULD BE SHOWING A WARNING SCREEN NOW")
              (`/Game/UI/WBP_RootLayout.PushWidgetToLayerStack` (`self.Root Layout`) (struct :`TagName` "UI.Layer.Menu") "/Game/UI/Menus/WBP_WarningScreen.WBP_WarningScreen_C"))
            ; After 2 Seconds reset the loop and check telemetry again
            (`KismetSystemLibrary.Delay` 2.0)
            (`self.Check Telemetry`)
            (`KismetArrayLibrary.Array_Clear` (`self.Warning Message`))))
        (else
          (`KismetSystemLibrary.Delay` 2.0)
          (`self.Check Telemetry`))))))

(event `Key|Escape`
  (params (Key :type "Key Structure"))
  (:`Pressed`
    (`KismetSystemLibrary.QuitGame` null "Quit")))

(event `InputAxisKey|MouseWheelAxis`
  (params (AxisValue :type "Float (single-precision)"))
  (bind _returnvalue (`KismetMathLibrary.SignOfFloat` AxisValue))
  (if (!= _returnvalue 0.0)
    (bind _returnvalue_2 (`KismetMaterialLibrary.GetScalarParameterValue` "/Game/UI/Map/MPC_MapData.MPC_MapData" "Zoom"))
    (`KismetMaterialLibrary.SetScalarParameterValue` "/Game/UI/Map/MPC_MapData.MPC_MapData" "Zoom" (`KismetMathLibrary.FClamp` (+ _returnvalue_2 (* _returnvalue -0.05)) 0.3 0.8))))

(fn `UserConstructionScript`)